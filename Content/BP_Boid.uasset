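; Boid actor that steers toward one optional target and away from another, without any neighbour flocking.
; Each tick it sums weighted Seek and Flee vectors, with Flee simply negating Seek.
; The sum blends into the previous force using Mass as the lerp alpha for inertia.
; The root then moves along that normalized direction at Speed, without sweep or rotation.
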(event `self.ReceiveTick`
  (params (DeltaSeconds :type "Float (single-precision)"))
  (bind _seektarget (`self.SeekTarget`))
  (bind _seektarget_0 (`self.SeekTarget_0`))
  (set `self.forces` (0.0 0.0 0.0))
  (`|ExecutionSequence`
    (:`then_0`
      (`/Engine/EditorBlueprintResources/StandardMacros.IsValid` _seektarget
        (:`Is Valid`
          (bind _force (`self.Seek` (`self.K2_GetActorLocation`) (`self.K2_GetActorLocation` _seektarget) (`self.SeekImpetu`)))
          (set `self.forces` (+ _force (`self.forces`))))))
    (:`then_1`
      (`/Engine/EditorBlueprintResources/StandardMacros.IsValid` _seektarget_0
        (:`Is Valid`
          (bind _force_2 (`self.Flee` (`self.K2_GetActorLocation`) (`self.K2_GetActorLocation` _seektarget_0) (`self.SeekImpetu_0`)))
          (set `self.forces` (+ _force_2 (`self.forces`))))))
    (:`then_2`
      (bind _output_get (set `self.oldForce` (`KismetMathLibrary.VLerp` (`self.forces`) (`self.oldForce`) (`self.Mass`))))
      (`SceneComponent.K2_AddWorldOffset` (`self.DefaultSceneRoot`) (* (`KismetMathLibrary.Normal` _output_get) (* (`self.speed`) DeltaSeconds)) false false))))

(fn `Flee`
  (params (myPos :type "Vector Structure") (TargetInput :type "Vector Structure") (Impetu :type "Float (double-precision)"))
  (returns (Force :type "Vector Structure"))
  (bind _force (`self.Seek` myPos TargetInput Impetu))
  (return (* _force -1.0)))

(fn `Seek`
  (params (MiPos :type "Vector Structure") (FinalPos :type "Vector Structure") (Impetu :type "Float (double-precision)"))
  (returns (force :type "Vector Structure"))
  (return (* (`KismetMathLibrary.Normal` (- FinalPos MiPos)) Impetu)))

(fn `UserConstructionScript`)