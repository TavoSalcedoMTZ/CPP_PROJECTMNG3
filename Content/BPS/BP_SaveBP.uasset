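; BP_SaveBP persists audio volume settings between sessions, restoring them on BeginPlay and saving them on EndPlay.
; Loading reads the "Save" slot and, if valid, casts it to SaveGameCustom and pushes Main, Music and SFX volumes into the AudioManager.
; Saving reads those three volumes from the AudioManager into a VolumeSettings struct on a freshly created SaveGameCustom, which overwrites the slot.
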(event `self.ReceiveBeginPlay`
  (`self.LoadVolumeSettings`))

(event `self.ReceiveEndPlay`
  (params (EndPlayReason :type "EEndPlayReason Enum" :default "Destroyed"))
  (`self.GuardarVolumeSettings`))

(fn `GuardarVolumeSettings`
  (bind _returnvalue (subsystem `AudioManager`))
  (bind _returnvalue_2 (`AudioManager.GetVolume` _returnvalue "Main"))
  (bind _returnvalue_3 (`AudioManager.GetVolume` _returnvalue "Music"))
  (bind _returnvalue_4 (`AudioManager.GetVolume` _returnvalue "SFX"))
  (bind _returnvalue_5 (`GameplayStatics.CreateSaveGameObject` "/Game/BPS/SaveGameCustom.SaveGameCustom_C"))
  (set `/Game/BPS/SaveGameCustom.VolumeSettings` (make `/Game/BPS/VS` _returnvalue_2 _returnvalue_3 _returnvalue_4) _returnvalue_5)
  (bind _returnvalue_6 (`GameplayStatics.SaveGameToSlot` _returnvalue_5 "Save"))
  (if _returnvalue_6
    (`KismetSystemLibrary.PrintString` "Save completo    ")))

(fn `LoadVolumeSettings`
  (bind _returnvalue (subsystem `AudioManager`))
  (bind _returnvalue_2 (`GameplayStatics.LoadGameFromSlot` "Save"))
  (`/Engine/EditorBlueprintResources/StandardMacros.IsValid` _returnvalue_2
    (:`Is Valid`
      (bind _assave_game_custom (cast `/Game/BPS/SaveGameCustom` _returnvalue_2))
      (bind (_mainvolume _musicvolume _sfx) (break `/Game/BPS/VS` (`/Game/BPS/SaveGameCustom.VolumeSettings` _assave_game_custom)))
      (`AudioManager.SetVolume` _returnvalue _mainvolume "Main")
      (`AudioManager.SetVolume` _returnvalue _musicvolume "Music")
      (`AudioManager.SetVolume` _returnvalue _sfx "SFX"))))

(fn `UserConstructionScript`)